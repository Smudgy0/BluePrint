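; AI enemy tank that aims its turret at the player and fires projectiles.
; Tick switches on a state enum: Aiming runs a one-shot timeline (key 3 resets it) that turns the turret and approaches the seen pawn, then switches to Fireing.
; Fireing tracks the player, spawns a projectile and returns to Aiming after a random delay.
; PawnSensing moves it toward noises; sight sets FollowPlayer, which Tick does not handle.
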(event `self.ReceiveTick`
  (params (DeltaSeconds :type "Float (single-precision)"))
  (bind _firingpos (`self.FiringPos`))
  (bind (_returnvalue_roll _returnvalue_pitch _returnvalue_yaw) (`KismetMathLibrary.BreakRotator` (`SceneComponent.K2_GetComponentRotation` (`self.Turret Hull`))))
  (bind (_returnvalue_roll_2 _returnvalue_pitch_2 _returnvalue_yaw_2) (`KismetMathLibrary.BreakRotator` (`KismetMathLibrary.FindLookAtRotation` (`SceneComponent.K2_GetComponentLocation` (`self.Turret Hull`)) (`self.K2_GetActorLocation` (`GameplayStatics.GetPlayerCharacter` 0)))))
  (bind (_returnvalue_roll_3 _returnvalue_pitch_3 _returnvalue_yaw_3) (`KismetMathLibrary.BreakRotator` (`KismetMathLibrary.FindLookAtRotation` (`SceneComponent.K2_GetComponentLocation` _firingpos) (`self.K2_GetActorLocation` (`GameplayStatics.GetPlayerPawn` 0)))))
  (switch `/Game/Scripts(BluePrints)/AI/E_AIStates` (`self.E_AIStates`)
    (:`NewEnumerator2`
      (`|ExecutionSequence`
        (:`then_0`
          (`SceneComponent.K2_SetWorldRotation` (`self.Turret Hull`) (`KismetMathLibrary.MakeRotator` 0.0 0.0 _returnvalue_yaw_3) false false)
          (`SceneComponent.K2_SetRelativeRotation` (`self.Rotator`) (`KismetMathLibrary.MakeRotator` 0.0 (- _returnvalue_pitch_3 90.0)) false false))
        (:`then_1`
          (if (not (`self.Fired`))
            (`|ExecutionSequence`
              (:`then_1`
                (`|SpawnActorFromClass` "/Game/Scripts(BluePrints)/Bullets/BP_Projectile.BP_Projectile_C" (`KismetMathLibrary.MakeTransform` (`SceneComponent.K2_GetComponentLocation` _firingpos) (`SceneComponent.K2_GetComponentRotation` _firingpos)) "AlwaysSpawn" "MultiplyWithRoot" null null)
                (set `self.Fired` true)
                (`KismetSystemLibrary.Delay` (`KismetMathLibrary.RandomFloatInRange` 1.0 2.0))
                (set `self.Fired` false)
                (set `self.E_AIStates` "NewEnumerator3")))))
        (:`then_2`
          (`KismetSystemLibrary.PrintString` "Bullet Spawned"))))
    (:`NewEnumerator3`
      (`/Engine/EditorBlueprintResources/StandardMacros.DoOnce` false :!label _label
        (:`Completed`
          (bind (_direction _newtrack_0) (`Timeline|Timeline` :!via `PlayFromStart`)
            (:`Update`
              (`SceneComponent.K2_SetWorldRotation` (`self.Turret Hull`) (`KismetMathLibrary.RLerp` (`KismetMathLibrary.MakeRotator` 0.0 0.0 _returnvalue_yaw) (`KismetMathLibrary.MakeRotator` 0.0 0.0 (- _returnvalue_yaw_2 90.0)) _newtrack_0 true) false false)
              (`|ExecutionSequence`
                (:`then_0`
                  (if (not (`self.Fired`))
                    (`|AIMoveTo` self (0.0 0.0 0.0) (stale `self.PawnSensing.OnSeePawn` Pawn) 1500.0
                      (:`OnSuccess`
                        (set `self.E_AIStates` "NewEnumerator3")))))
                (:`then_1`
                  (`KismetSystemLibrary.RetriggerableDelay` 0.6)
                  (`MovementComponent.StopMovementImmediately` (`self.CharacterMovement`)))))
            (:`Finished`
              (`KismetSystemLibrary.Delay` 1.0)
              (set `self.E_AIStates` "NewEnumerator2"))))))))

(event `Key|Three`
  (params (Key :type "Key Structure"))
  (:`Pressed`
    (goto _label :!via `Reset`)))

(event `self.PawnSensing.OnSeePawn`
  (params (Pawn :type "Pawn Object Reference"))
  (set `self.E_AIStates` "NewEnumerator1"))

(event `self.PawnSensing.OnHearNoise`
  (params (Instigator :type "Pawn Object Reference") (Location :type "Vector Structure (by ref)") (Volume :type "Float (single-precision)"))
  (`|ExecutionSequence`
    (:`then_0`
      (`|AIMoveTo` self (0.0 0.0 0.0) Instigator))
    (:`then_1`
      (`KismetSystemLibrary.RetriggerableDelay` 0.6)
      (`MovementComponent.StopMovementImmediately` (`self.CharacterMovement`)))))

(fn `UserConstructionScript`)
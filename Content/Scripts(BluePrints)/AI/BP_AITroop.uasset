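; BP_AITroop is an enemy AI troop that chases what it senses and deals repeated damage to the player up close.
; PawnSensing sight and hearing store a target and start AIMoveTo toward it.
; Sphere overlap with the first-person character enables the DamagePlayer macro on Tick, where a gate and delay limit hits to one per second.
; Incoming damage lowers clamped Health, prints it, and destroys the troop at zero.
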(event `self.ReceiveTick`
  (params (DeltaSeconds :type "Float (single-precision)"))
  (if (== (stale `self.Sphere.OnComponentEndOverlap` OtherActor) (`self.Other Actor`))
    (`self.DamagePlayer` :!label _label)))

(event `self.Sphere.OnComponentEndOverlap`
  (params (OverlappedComponent :type "PrimitiveComponent Object Reference") (OtherActor :type "Actor Object Reference") (OtherComp :type "PrimitiveComponent Object Reference") (OtherBodyIndex :type Integer))
  (goto _label :!via `End Overlap`))

(event `self.Sphere.OnComponentBeginOverlap`
  (params (OverlappedComponent :type "PrimitiveComponent Object Reference") (OtherActor :type "Actor Object Reference") (OtherComp :type "PrimitiveComponent Object Reference") (OtherBodyIndex :type Integer) (bFromSweep :type Boolean) (SweepResult :type "HitResult Structure (by ref)"))
  (set `self.DamagingPlayer` true)
  (bind _asbp_first_person_character (cast `/Game/FirstPerson/Blueprints/BP_FirstPersonCharacter` OtherActor))
  (set `self.Other Actor` _asbp_first_person_character))

(event `self.PawnSensing.OnSeePawn`
  (params (Pawn :type "Pawn Object Reference"))
  (set `self.Other Actor` Pawn)
  (`|AIMoveTo` self (0.0 0.0 0.0) (`self.Other Actor`) :!label _label_2))

(event `self.PawnSensing.OnHearNoise`
  (params (Instigator :type "Pawn Object Reference") (Location :type "Vector Structure (by ref)") (Volume :type "Float (single-precision)"))
  (set `self.Other Actor` Instigator)
  (goto _label_2))

(event `self.ReceiveAnyDamage`
  (params (Damage :type "Float (single-precision)") (DamageType :type "DamageType Object Reference") (InstigatedBy :type "Controller Object Reference") (DamageCauser :type "Actor Object Reference"))
  (bind _output_get (set `self.Health` (`KismetMathLibrary.FClamp` (- (`self.Health`) Damage) 0.0 (`self.MaxHP`))))
  (`KismetSystemLibrary.PrintString` (`KismetStringLibrary.Conv_DoubleToString` _output_get))
  (if (== _output_get 0.0)
    (`self.K2_DestroyActor`)))

(event `self.PawnSensing.OnComponentActivated`
  (params (Component :type "ActorComponent Object Reference") (bReset :type Boolean))
  (`KismetSystemLibrary.PrintString` "2"))

(fn `UserConstructionScript`)
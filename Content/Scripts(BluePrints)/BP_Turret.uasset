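; BP_Turret is a turret that constantly tracks the player pawn and fires BP_Projectile actors, with no range or line-of-sight check.
; Each tick it yaws the Cube and pitches the Cylinder from a look-at rotation between the Arrow and the player.
; The Arrow supplies the projectile spawn location and rotation.
; A Fired flag with a short random delay gates each shot, and a PointLight briefly flashes on firing.
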(event `self.ReceiveTick`
  (params (DeltaSeconds :type "Float (single-precision)"))
  (bind _pointlight (`self.PointLight`))
  (bind _arrow (`self.Arrow`))
  (bind (_returnvalue_roll _returnvalue_pitch _returnvalue_yaw) (`KismetMathLibrary.BreakRotator` (`KismetMathLibrary.FindLookAtRotation` (`SceneComponent.K2_GetComponentLocation` (`self.Arrow`)) (`self.K2_GetActorLocation` (`GameplayStatics.GetPlayerPawn` 0)))))
  (`|ExecutionSequence`
    (:`then_0`
      (`SceneComponent.K2_SetWorldRotation` (`self.Cube`) (`KismetMathLibrary.MakeRotator` 0.0 0.0 _returnvalue_yaw) false false)
      (`SceneComponent.K2_SetRelativeRotation` (`self.Cylinder`) (`KismetMathLibrary.MakeRotator` 0.0 (- _returnvalue_pitch 90.0)) false false))
    (:`then_1`
      (if (not (`self.Fired`))
        (`|ExecutionSequence`
          (:`then_0`
            (`SceneComponent.SetVisibility` _pointlight true false)
            (`KismetSystemLibrary.Delay` 0.2)
            (`SceneComponent.SetVisibility` _pointlight false false))
          (:`then_1`
            (`|SpawnActorFromClass` "/Game/Scripts(BluePrints)/BP_Projectile.BP_Projectile_C" (`KismetMathLibrary.MakeTransform` (`SceneComponent.K2_GetComponentLocation` _arrow) (`SceneComponent.K2_GetComponentRotation` _arrow)) "Undefined" "MultiplyWithRoot" null null)
            (set `self.Fired` true)
            (`KismetSystemLibrary.Delay` (`KismetMathLibrary.RandomFloatInRange` 0.5 1.0))
            (set `self.Fired` false)))))))

(fn `UserConstructionScript`)
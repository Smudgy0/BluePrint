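; BP_MG is a twin-muzzle machine gun turret that tracks the player pawn and fires projectiles automatically.
; Each Tick, beyond MinFiringRange, it prints the distance and aims from the first arrow, yawing the Cube and pitching the Cylinder.
; Regardless of range, both arrows independently spawn BP_MGProjectile, each gated by a flag reset after a short random delay.
; Each shot briefly shows that muzzle's point light as a flash.
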(event `self.ReceiveTick`
  (params (DeltaSeconds :type "Float (single-precision)"))
  (bind _returnvalue (`KismetMathLibrary.RandomFloatInRange` 0.1 0.4))
  (bind _pointlight (`self.PointLight`))
  (bind _arrow1 (`self.Arrow1`))
  (bind _pointlight1 (`self.PointLight1`))
  (bind _arrow (`self.Arrow`))
  (bind _returnvalue_2 (`KismetMathLibrary.Vector_Distance` (`self.K2_GetActorLocation` (`GameplayStatics.GetPlayerPawn` 0)) (`self.K2_GetActorLocation`)))
  (bind (_returnvalue_roll _returnvalue_pitch _returnvalue_yaw) (`KismetMathLibrary.BreakRotator` (`KismetMathLibrary.FindLookAtRotation` (`SceneComponent.K2_GetComponentLocation` (`self.Arrow`)) (`self.K2_GetActorLocation` (`GameplayStatics.GetPlayerPawn` 0)))))
  (`|ExecutionSequence`
    (:`then_0`
      ;[1 1 1] Turret Rotation
      (if (> _returnvalue_2 (`self.MinFiringRange`))
        (`KismetSystemLibrary.PrintString` (`KismetStringLibrary.Conv_DoubleToString` _returnvalue_2))
        (`SceneComponent.K2_SetWorldRotation` (`self.Cube`) (`KismetMathLibrary.MakeRotator` 0.0 0.0 _returnvalue_yaw) false false)
        (`SceneComponent.K2_SetRelativeRotation` (`self.Cylinder`) (`KismetMathLibrary.MakeRotator` 0.0 (- _returnvalue_pitch 90.0)) false false)))
    (:`then_1`
      (`|ExecutionSequence`
        (:`then_0`
          (if (not (`self.Fired`))
            (`|ExecutionSequence`
              (:`then_0`
                (`SceneComponent.SetVisibility` _pointlight true false)
                (`KismetSystemLibrary.Delay` 0.2)
                (`SceneComponent.SetVisibility` _pointlight false false))
              (:`then_1`
                (`|SpawnActorFromClass` "/Game/Scripts(BluePrints)/BP_MGProjectile.BP_MGProjectile_C" (`KismetMathLibrary.MakeTransform` (`SceneComponent.K2_GetComponentLocation` _arrow) (`SceneComponent.K2_GetComponentRotation` _arrow)) "AlwaysSpawn" "MultiplyWithRoot" null null)
                (set `self.Fired` true)
                (`KismetSystemLibrary.Delay` _returnvalue)
                (set `self.Fired` false)))))
        (:`then_1`
          (if (not (`self.Fired_2`))
            (`|ExecutionSequence`
              (:`then_0`
                (`SceneComponent.SetVisibility` _pointlight1 true false)
                (`KismetSystemLibrary.Delay` 0.2)
                (`SceneComponent.SetVisibility` _pointlight1 false false))
              (:`then_1`
                (`|SpawnActorFromClass` "/Game/Scripts(BluePrints)/BP_MGProjectile.BP_MGProjectile_C" (`KismetMathLibrary.MakeTransform` (`SceneComponent.K2_GetComponentLocation` _arrow1) (`SceneComponent.K2_GetComponentRotation` _arrow1)) "AlwaysSpawn" "MultiplyWithRoot" null null)
                (set `self.Fired_2` true)
                (`KismetSystemLibrary.Delay` _returnvalue)
                (set `self.Fired_2` false)))))))))

(fn `UserConstructionScript`)
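; Turret actor that constantly tracks the player and fires BP_Projectile at them.
; Each Tick it yaws the Cube and pitches the Cylinder using look-at rotations from the Arrow to the player pawn.
; It fires from the Arrow only while sitting higher than the player, unless IgnoreHeight is set.
; Each shot briefly flashes a PointLight, with a Fired flag and random Delay forming the cooldown.
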(event `self.ReceiveTick`
  (params (DeltaSeconds :type "Float (single-precision)"))
  (bind (_returnvalue_x _returnvalue_y _returnvalue_z) (`KismetMathLibrary.BreakVector` (`self.K2_GetActorLocation`)))
  (bind _pointlight (`self.PointLight`))
  (bind _arrow (`self.Arrow`))
  (bind (_returnvalue_x_2 _returnvalue_y_2 _returnvalue_z_2) (`KismetMathLibrary.BreakVector` (`self.K2_GetActorLocation` (`GameplayStatics.GetPlayerPawn` 0))))
  (bind (_returnvalue_roll _returnvalue_pitch _returnvalue_yaw) (`KismetMathLibrary.BreakRotator` (`KismetMathLibrary.FindLookAtRotation` (`SceneComponent.K2_GetComponentLocation` (`self.Arrow`)) (`self.K2_GetActorLocation` (`GameplayStatics.GetPlayerPawn` 0)))))
  (`|ExecutionSequence`
    (:`then_0`
      ;[0 0.1796 1] Set rotation of the turret to be facing the player at all times
      (`SceneComponent.K2_SetWorldRotation` (`self.Cube`) (`KismetMathLibrary.MakeRotator` 0.0 0.0 _returnvalue_yaw) false false)
      (`SceneComponent.K2_SetRelativeRotation` (`self.Cylinder`) (`KismetMathLibrary.MakeRotator` 0.0 (- _returnvalue_pitch 90.0)) false false))
    (:`then_1`
      ;[0 1 0.02214] Checks if the turret is not on cooldown before firing
      (if (or (> _returnvalue_z _returnvalue_z_2) (`self.IgnoreHeight`))
        (if (not (`self.Fired`))
          (`|ExecutionSequence`
            (:`then_0`
              ;[1 0.8104 0] Light flash for firing
              (`SceneComponent.SetVisibility` _pointlight true false)
              (`KismetSystemLibrary.Delay` 0.2)
              (`SceneComponent.SetVisibility` _pointlight false false))
            (:`then_1`
              ;[1 0 0] Spawn Bullet And then set fired to true for 0.5 to 1 second (how long it takes to fire again)
              (`|SpawnActorFromClass` "/Game/Scripts(BluePrints)/Bullets/BP_Projectile.BP_Projectile_C" (`KismetMathLibrary.MakeTransform` (`SceneComponent.K2_GetComponentLocation` _arrow) (`SceneComponent.K2_GetComponentRotation` _arrow)) "Undefined" "MultiplyWithRoot" null null)
              (set `self.Fired` true)
              (`KismetSystemLibrary.Delay` (`KismetMathLibrary.RandomFloatInRange` 0.5 1.0))
              (set `self.Fired` false))))))))

(fn `UserConstructionScript`)
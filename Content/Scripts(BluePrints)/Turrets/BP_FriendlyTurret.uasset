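; Friendly twin-barrel turret that tracks BP_Projectile actors and fires friendly machine-gun projectiles.
; BulletTargeter's OnSeePawn casts the seen pawn's parent actor to BP_Projectile, then yaws Cube and pitches Cylinder toward it.
; Aiming runs only while the player is beyond MinFiringRange from the turret.
; Tick fires both barrels continuously, independent of targeting, each gated by its own randomized Delay cooldown with a brief muzzle-light flash.
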(event `self.BulletTargeter.OnSeePawn`
  (params (Pawn :type "Pawn Object Reference"))
  (bind _asbp_projectile (cast `/Game/Scripts(BluePrints)/Bullets/BP_Projectile` (`self.GetParentActor` Pawn)))
  ;[1 1 1] Turret Rotation
  (if (> (`KismetMathLibrary.Vector_Distance` (`self.K2_GetActorLocation` (`GameplayStatics.GetPlayerPawn` 0)) (`self.K2_GetActorLocation`)) (`self.MinFiringRange`))
    (bind (_returnvalue_roll _returnvalue_pitch _returnvalue_yaw) (`KismetMathLibrary.BreakRotator` (`KismetMathLibrary.FindLookAtRotation` (`SceneComponent.K2_GetComponentLocation` (`self.Arrow`)) (`SceneComponent.K2_GetComponentLocation` (`Actor.RootComponent` _asbp_projectile)))))
    (`SceneComponent.K2_SetWorldRotation` (`self.Cube`) (`KismetMathLibrary.MakeRotator` 0.0 0.0 _returnvalue_yaw) false false)
    (`SceneComponent.K2_SetRelativeRotation` (`self.Cylinder`) (`KismetMathLibrary.MakeRotator` 0.0 (- _returnvalue_pitch 90.0)) false false)))

(event `self.ReceiveTick`
  (params (DeltaSeconds :type "Float (single-precision)"))
  (bind _returnvalue (`KismetMathLibrary.RandomFloatInRange` 0.5 0.6))
  (bind _pointlight (`self.PointLight`))
  (bind _arrow1 (`self.Arrow1`))
  (bind _pointlight1 (`self.PointLight1`))
  (bind _arrow (`self.Arrow`))
  (`|ExecutionSequence`
    (:`then_1`
      (`|ExecutionSequence`
        (:`then_0`
          (if (not (`self.Fired`))
            (`|ExecutionSequence`
              (:`then_0`
                (`SceneComponent.SetVisibility` _pointlight true false)
                (`KismetSystemLibrary.Delay` 0.2)
                (`SceneComponent.SetVisibility` _pointlight false false))
              (:`then_1`
                (`|SpawnActorFromClass` "/Game/Scripts(BluePrints)/Bullets/BP_FriendMGProjectile1.BP_FriendMGProjectile1_C" (`KismetMathLibrary.MakeTransform` (`SceneComponent.K2_GetComponentLocation` _arrow) (`SceneComponent.K2_GetComponentRotation` _arrow)) "AlwaysSpawn" "MultiplyWithRoot" null null)
                (set `self.Fired` true)
                (`KismetSystemLibrary.Delay` _returnvalue)
                (set `self.Fired` false)))))
        (:`then_1`
          (if (not (`self.Fired_2`))
            (`|ExecutionSequence`
              (:`then_0`
                (`SceneComponent.SetVisibility` _pointlight1 true false)
                (`KismetSystemLibrary.Delay` 0.2)
                (`SceneComponent.SetVisibility` _pointlight1 false false))
              (:`then_1`
                (`|SpawnActorFromClass` "/Game/Scripts(BluePrints)/Bullets/BP_FriendMGProjectile1.BP_FriendMGProjectile1_C" (`KismetMathLibrary.MakeTransform` (`SceneComponent.K2_GetComponentLocation` _arrow1) (`SceneComponent.K2_GetComponentRotation` _arrow1)) "AlwaysSpawn" "MultiplyWithRoot" null null)
                (set `self.Fired_2` true)
                (`KismetSystemLibrary.Delay` _returnvalue)
                (set `self.Fired_2` false)))))))))

(fn `UserConstructionScript`)